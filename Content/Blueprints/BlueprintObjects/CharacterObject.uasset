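; CharacterObject is the player-controlled 2D sprite character, driven by MoveUp and MoveRight axis inputs.
; On BeginPlay it has the first player controller possess it and switches the view to a referenced main camera.
; MoveUp moves along the collision box's right vector and MoveRight along its forward vector.
; MoveRight also swaps the Paper2D sprite at full positive or negative input, leaving it unchanged otherwise.
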(event `self.ReceiveBeginPlay`
  (`Controller.Possess` (`GameplayStatics.GetPlayerController` 0) self)
  (`PlayerController.SetViewTargetWithBlend` (`GameplayStatics.GetPlayerController` 0) (`self.MainCameraReference`) 0.0 "VTBlend_Linear" 0.0 false))

(event `InputAxis|MoveUp`
  (params (AxisValue :type "Float (single-precision)"))
  (`self.AddMovementInput` (`SceneComponent.GetRightVector` (`self.CollisionBox`)) AxisValue))

(event `InputAxis|MoveRight`
  (params (AxisValue :type "Float (single-precision)"))
  (`self.AddMovementInput` (`SceneComponent.GetForwardVector` (`self.CollisionBox`)) AxisValue)
  (if (== AxisValue 1.0)
    (`PaperSpriteComponent.SetSprite` (`self.CharacterSprite`) "/Game/Sprites/NewPaperSprite.NewPaperSprite")
    (elif (== AxisValue -1.0)
      (`PaperSpriteComponent.SetSprite` (`self.CharacterSprite`) "/Game/Sprites/NewPaperSprite1.NewPaperSprite1"))))

(fn `UserConstructionScript`)