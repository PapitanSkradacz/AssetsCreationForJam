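; DetectionSensor is a sphere-trigger actor that reports detection of the player's CharacterObject to that character.
; It finds the player at BeginPlay, then on every Tick while overlapping sends a detection amount of frame time scaled by its weight.
; Begin overlap also sends its configured detection object if the player is inside.
; End overlap sends an empty value without checking which actor left.
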(event `self.ReceiveBeginPlay`
  (bind _returnvalue (`GameplayStatics.GetActorOfClass` "/Game/Blueprints/BlueprintObjects/CharacterObject.CharacterObject_C"))
  (set `self.PlayerActor` _returnvalue))

(event `self.ReceiveTick`
  (params (DeltaSeconds :type "Float (single-precision)"))
  (if (`PrimitiveComponent.IsOverlappingActor` (`self.Sphere`) (`self.PlayerActor`))
    (message `/Game/Blueprints/InterfacesETC/Detection_Interface.SendDetection` (`self.PlayerActor`) (* DeltaSeconds (`self.ThisMarkerDetectionWeight`)))))

(event `self.Sphere.OnComponentBeginOverlap`
  (params (OverlappedComponent :type "PrimitiveComponent Object Reference") (OtherActor :type "Actor Object Reference") (OtherComp :type "PrimitiveComponent Object Reference") (OtherBodyIndex :type Integer) (bFromSweep :type Boolean) (SweepResult :type "HitResult Structure (by ref)"))
  (if (`PrimitiveComponent.IsOverlappingActor` (`self.Sphere`) (`self.PlayerActor`))
    (message `/Game/Blueprints/InterfacesETC/Detection_Interface.SendDetectionObject` (`self.PlayerActor`) (`self.DetectionObjectItTriggers`))))

(event `self.Sphere.OnComponentEndOverlap`
  (params (OverlappedComponent :type "PrimitiveComponent Object Reference") (OtherActor :type "Actor Object Reference") (OtherComp :type "PrimitiveComponent Object Reference") (OtherBodyIndex :type Integer))
  (message `/Game/Blueprints/InterfacesETC/Detection_Interface.SendDetectionObject` (`self.PlayerActor`) (`self.emptyVar`)))

(fn `UserConstructionScript`)